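; BP_PlayerCharacter01 is a side-view player character with Enhanced Input movement and jumping.
; On BeginPlay it adds the IMC_Player01 mapping context to player 0's input subsystem.
; The move action, gated by CanMove, drives movement along world X and flips PlayerSprite by rotation to match facing, printing a debug message when locked.
; The jump action starts and stops the built-in Character jump.
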(event Input|EnhancedActionEvents|EnhancedInputActionIA_move01
  (params (ActionValue :type Vector%202D%20Structure) (ElapsedSeconds :type Float%20%28double-precision%29) (TriggeredSeconds :type Float%20%28double-precision%29) (InputAction :type Input%20Action%20Object%20Reference :default "/Game/my15/Input/IA_move01.IA_move01"))
  (bind _x (Math|Vector2D|BreakVector2D ActionValue))
  (bind _playersprite (Variables|Default|GetPlayerSprite))
  (if (Variables|Default|GetCanMove)
    (if (> _x 0.0)
      (Variables|Default|SetIsFacingRight true)
      (else
        (Variables|Default|SetIsFacingRight false)))
    (Pawn|Input|AddMovementInput "1.000000,0.000000,0.000000" _x false)
    (if (Variables|Default|GetIsFacingRight)
      (Transformation|SetRelativeRotation _playersprite "0, 0, 0" false false)
      (else
        (Transformation|SetRelativeRotation _playersprite "0.000000,180.000000,0.000000" false false)))
    (else
      (Development|PrintString "Move Locked"))))

(event Input|EnhancedActionEvents|EnhancedInputActionIA_Jump01
  (params (ActionValue :type Boolean) (ElapsedSeconds :type Float%20%28double-precision%29) (TriggeredSeconds :type Float%20%28double-precision%29) (InputAction :type Input%20Action%20Object%20Reference :default "/Game/my15/Input/IA_Jump01.IA_Jump01"))
  (:Started
    (Character|Jump))
  (:Completed
    (Character|StopJumping)))

(event EventBeginPlay
  (Input|AddMappingContext (PlayerController|LocalPlayerSubsystems|GetEnhancedInputLocalPlayerSubsystem (Game|GetPlayerController 0)) "/Game/my15/Input/IMC_Player01.IMC_Player01" 0 "(bIgnoreAllPressedKeysUntilRelease=True,bForceImmediately=False,bNotifyUserSettings=False)"))

(event Collision|EventActorBeginOverlap
  (params (OtherActor :type Actor%20Object%20Reference)))

(event EventTick
  (params (DeltaSeconds :type Float%20%28single-precision%29)))

(fn ConstructionScript)
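; Parallax backdrop actor that shifts three layers horizontally as the player character moves, creating depth in the scene.
; BeginPlay stores the player's starting X, and every Tick calls UpdateParallax to measure the X displacement from that point.
; UpdateParallax scales that displacement by separate far, mid and near factors to set each layer's relative X, with fixed depth offsets in Y and a lowered mid layer.
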(event EventBeginPlay
  (Variables|Default|SetPlayStartX (.X (Math|Vector|BreakVector (Transformation|GetActorLocation (Game|GetPlayerCharacter 0))))))

(event Collision|EventActorBeginOverlap
  (params (OtherActor :type Actor%20Object%20Reference)))

(event EventTick
  (params (DeltaSeconds :type Float%20%28single-precision%29))
  (CallFunction|UpdateParallax))

(fn ConstructionScript)

(fn UpdateParallax
  (Variables|Default|SetDeltaX (- (.X (Math|Vector|BreakVector (Transformation|GetActorLocation (Game|GetPlayerCharacter 0)))) (Variables|Default|GetPlayStartX)))
  (Utilities|FlowControl|Sequence
    (:then_0
      (Transformation|SetRelativeLocation (Variables|Default|GetSP_Far) (Math|Vector|MakeVector (+ (Variables|Default|GetXstart) (* (Variables|Default|GetDeltaX) (Variables|Default|GetFarGB))) (+ (Variables|Default|GetYstart) -2e+02) (Variables|Default|GetZstart)) false false))
    (:then_1
      (Transformation|SetRelativeLocation (Variables|Default|GetSP_Mid) (Math|Vector|MakeVector (+ (Variables|Default|GetXstart) (* (Variables|Default|GetDeltaX) (Variables|Default|GetMidGB))) (+ (Variables|Default|GetYstart) -1e+02) (- (Variables|Default|GetZstart) 1e+02)) false false))
    (:then_2
      (Transformation|SetRelativeLocation (Variables|Default|GetSP_near) (Math|Vector|MakeVector (+ (Variables|Default|GetXstart) (* (Variables|Default|GetDeltaX) (Variables|Default|GetNearGB))) (Variables|Default|GetYstart) (Variables|Default|GetZstart)) false false))))